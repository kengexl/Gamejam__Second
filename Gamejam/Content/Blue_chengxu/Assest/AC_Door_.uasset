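; Interactable hinged door that swings open 90 degrees either way depending on the player's side, with an overlay-material outline for highlighting.
; Front and Back trigger overlaps set the Where flag, which Interaction uses to pick one of two timelines rotating DoorOpenDot's yaw.
; Each direction's FlipFlop alternates play and reverse, while IsA and IsA0 record its state so an open door closes the way it opened.
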(event OnComponentBeginOverlap(Fornt)
  (params (OverlappedComponent :type Primitive%20Component%20Object%20Reference) (OtherActor :type Actor%20Object%20Reference) (OtherComp :type Primitive%20Component%20Object%20Reference) (OtherBodyIndex :type Integer) (bFromSweep :type Boolean) (SweepResult :type Hit%20Result%20Structure%20%28by%20ref%29))
  (if (== OtherActor (Game|GetPlayerCharacter 0))
    (Variables|Default|SetWhere false)))

(event OnComponentEndOverlap(Fornt)
  (params (OverlappedComponent :type Primitive%20Component%20Object%20Reference) (OtherActor :type Actor%20Object%20Reference) (OtherComp :type Primitive%20Component%20Object%20Reference) (OtherBodyIndex :type Integer))
  (if (== OtherActor (Game|GetPlayerCharacter 0))
    (Variables|Default|SetWhere false)))

(event OnComponentBeginOverlap(Back)
  (params (OverlappedComponent :type Primitive%20Component%20Object%20Reference) (OtherActor :type Actor%20Object%20Reference) (OtherComp :type Primitive%20Component%20Object%20Reference) (OtherBodyIndex :type Integer) (bFromSweep :type Boolean) (SweepResult :type Hit%20Result%20Structure%20%28by%20ref%29))
  (if (== (Game|GetPlayerCharacter 0) OtherActor)
    (Variables|Default|SetWhere true)))

(event OnComponentEndOverlap(Back)
  (params (OverlappedComponent :type Primitive%20Component%20Object%20Reference) (OtherActor :type Actor%20Object%20Reference) (OtherComp :type Primitive%20Component%20Object%20Reference) (OtherBodyIndex :type Integer))
  (if (== (Game|GetPlayerCharacter 0) OtherActor)
    (Variables|Default|SetWhere false)))

(event EventBeginPlay)

(event Collision|EventActorBeginOverlap
  (params (OtherActor :type Actor%20Object%20Reference)))

(event EventOutlineClear
  ;[1 1 1] 可交互物品的描边添加与删除
  (Rendering|Material|SetOverlayMaterial (Variables|Default|GetStaticMesh) 0 :!class /Script/Engine.MeshComponent))

(event EventOutline
  ;[1 1 1] 可交互物品的描边添加与删除
  (Rendering|Material|SetOverlayMaterial (Variables|Default|GetStaticMesh) "/Game/Texture/MI_Outline.MI_Outline" :!class /Script/Engine.MeshComponent))

(event EventInteraction
  (if (== (Variables|Default|GetIs%20A) (Variables|Default|GetIs%20A_0))
    (if (Variables|Default|GetWhere)
      (bind _isa (Utilities|FlowControl|FlipFlop :!label _label)
        (:A
          (bind _0to1 (Timeline|时间轴 PlayFromStart)
            (:Update
              (Variables|Default|SetIs%20A _isa)
              (Transformation|SetRelativeRotation (Variables|Default|GetDoor_Open_Dot) (Math|Rotator|MakeRotator 0.0 0.0 (Math|Float|Lerp 0.0 9e+01 _0to1)) false false))))
        (:B
          (Timeline|时间轴 Reverse)))
      (else
        (bind _isa_2 (Utilities|FlowControl|FlipFlop :!label _label_2)
          (:A
            (bind _0to1_2 (Timeline|时间轴_0 PlayFromStart)
              (:Update
                (Variables|Default|SetIs%20A_0 _isa_2)
                (Transformation|SetRelativeRotation (Variables|Default|GetDoor_Open_Dot) (Math|Rotator|MakeRotator 0.0 0.0 (Math|Float|Lerp 0.0 -9e+01 _0to1_2)) false false))))
          (:B
            (Timeline|时间轴_0 Reverse)))))
    (elif (Variables|Default|GetIs%20A)
      (goto _label)
      (elif (Variables|Default|GetIs%20A_0)
        (goto _label_2)))))

(fn ConstructionScript)